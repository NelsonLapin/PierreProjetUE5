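; BP_EnemyAI is an enemy that wanders, chases the player on sight and deals damage on contact.
; It loops AI moves to random reachable points with a short pause between them.
; Pawn sensing sends it toward the cached player, with a retriggerable delay resuming wandering once sightings stop.
; Its collision box damages the player and destroys the enemy, while an unconnected level-open node marks an unfinished death menu.
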(event OnSeePawn(PawnSensing)
  (params (Pawn :type Pawn%20Object%20Reference))
  ;[1 1 1] Purchase Player
  (Utilities|FlowControl|Sequence
    (:then_0
      (AI|AIMoveTo self "0, 0, 0" (Variables|Default|GetAs%20BP%20Player) 5.0 false))
    (:then_1
      ;;[1 1 1] if doesn't see player
      (Utilities|FlowControl|RetriggerableDelay 2.0)
      (CallFunction|RandomWalk))))

(event OnComponentBeginOverlap(BoxCollision)
  (params (OverlappedComponent :type Primitive%20Component%20Object%20Reference) (OtherActor :type Actor%20Object%20Reference) (OtherComp :type Primitive%20Component%20Object%20Reference) (OtherBodyIndex :type Integer) (bFromSweep :type Boolean) (SweepResult :type Hit%20Result%20Structure%20%28by%20ref%29))
  ;[1 1 1] Death Trigger
  (if (== OtherActor (Variables|Default|GetAs%20BP%20Player))
    (Game|Damage|ApplyDamage (Variables|Default|GetAs%20BP%20Player) 1.0 0 0)
    (Actor|DestroyActor)))

(event Custom|Random%20Walk
  ;[1 1 1] Random Walk
  (Variables|Default|SetDetected? false)
  (AI|AIMoveTo self (.RandomLocation (AI|Navigation|GetRandomReachablePointinRadius (Transformation|GetActorLocation) 2e+03 0 0)) 0 5.0 false
    (:then
      (Utilities|FlowControl|Delay 3.0)
      (CallFunction|RandomWalk))))

(event EventBeginPlay
  ;[1 1 1] Begin Play
  (CallFunction|RandomWalk)
  (CallFunction|GetBlueprints))

(fn ConstructionScript)

(fn GetBlueprints
  (bind _asbp_player (Utilities|Casting|CastToBP_Player (Game|GetPlayerCharacter 0)))
  (Variables|Default|SetAs%20BP%20Player _asbp_player))