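; Level 3 door actor that opens once the player has exactly three collectibles.
; On BeginPlay it caches the BP_Player reference from the player character, then calls DoorMovement.
; DoorMovement polls the player's collectible count, retrying after a short delay until it matches.
; It then raises the static mesh along relative Z in a single instant jump, without interpolation.
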(event Custom|Door%20Movement
  (bind _staticmesh (Variables|Default|GetStaticMesh))
  (bind _relativelocation (Variables|/Script/Engine.SceneComponent|GetRelativeLocation _staticmesh))
  (bind _returnvalue (+ (.z _relativelocation) 2.5e+02))
  (if (== 3 (Variables|/Game/Player/BP_Player.BP_Player_C|GetNbCollectibles (Variables|Default|GetAs%20BP%20Player)))
    (Transformation|SetRelativeLocation _staticmesh (Math|Vector|MakeVector (.x _relativelocation) (.y _relativelocation) _returnvalue) false false)
    (if (== _returnvalue (.z (Variables|/Script/Engine.SceneComponent|GetRelativeLocation _staticmesh)))
      _)
    (else
      (Utilities|FlowControl|Delay 0.2)
      (CallFunction|DoorMovement))))

(event EventBeginPlay
  (CallFunction|GetBlueprints)
  (CallFunction|DoorMovement))

(fn ConstructionScript)

(fn GetBlueprints
  (bind _asbp_player (Utilities|Casting|CastToBP_Player (Game|GetPlayerCharacter 0)))
  (Variables|Default|SetAs%20BP%20Player _asbp_player))