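; Finish trigger for Level 1 that shows the win screen and moves the game on to Pierre_Level_2.
; Any overlap with its Box, with no check on the overlapping actor, adds the UI_YouWin_Lvl1 widget, plays a win sound and opens the next level after a short delay.
; The same overlap clears the Level 1 chrono-running flag on the BPGM_Player game mode without waiting for that delay.
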(event OnComponentBeginOverlap(Box)
  (params (OverlappedComponent :type Primitive%20Component%20Object%20Reference) (OtherActor :type Actor%20Object%20Reference) (OtherComp :type Primitive%20Component%20Object%20Reference) (OtherBodyIndex :type Integer) (bFromSweep :type Boolean) (SweepResult :type Hit%20Result%20Structure%20%28by%20ref%29))
  (bind _asbpgm_player (Utilities|Casting|CastToBPGM_Player (Game|GetGameMode)))
  (Utilities|FlowControl|Sequence
    (:then_0
      (bind _returnvalue (UserInterface|CreateWidget "/Game/Map/UI_YouWin_Lvl1.UI_YouWin_Lvl1_C"))
      (UserInterface|Viewport|AddtoViewport _returnvalue 0)
      (Audio|PlaySound2D "/Game/Sound/SoundEffect/WinLevel.WinLevel" 1.0 1.0 0.0 0 0)
      (Utilities|FlowControl|Delay 3.0)
      (Game|OpenLevel(byName) "Pierre_Level_2"))
    (:then_1
      (if (Variables|/Game/System/BPGM_Player.BPGM_Player_C|GetChronoRunning_Level1 _asbpgm_player)
        (Variables|/Game/System/BPGM_Player.BPGM_Player_C|SetChronoRunning_Level1 _asbpgm_player false)))))

(fn ConstructionScript)